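; BP_Barrel is an explosive barrel that detonates when its health runs out and is set up to respawn.
; HealthComp's OnHealthChanged event triggers a one-time blast, guarded by the Blust flag, that deals radial damage and plays an explosion sound.
; It then sets a short lifespan and, after an equal Delay, spawns a replacement at its location, so the respawn races the actor's own destruction.
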(event `self.ReceiveTick`
  (params (DeltaSeconds :type "Float (single-precision)")))

(event `self.ReceiveBeginPlay`)

(event `self.HealthComp.OnHealthChanged`
  (params (HealthComp :type "SHealthComponent Object Reference") (Health :type "Float (single-precision)") (HealthDelta :type "Float (single-precision)") (DamageType :type "DamageType Object Reference") (InstigatedBy :type "Controller Object Reference") (DamageCauser :type "Actor Object Reference"))
  (bind _returnvalue (`self.K2_GetActorLocation`))
  (if (<= Health 0.0)
    (if (not (`self.blust`))
      (`|ExecutionSequence`
        (:`then_0`
          (`GameplayStatics.ApplyRadialDamage` :`BaseDamage` 200.0 :`Origin` _returnvalue :`DamageRadius` 100.0 :`DamageTypeClass` (`GameplayStatics.GetObjectClass` DamageType) :`DamageCauser` self :`InstigatedByController` null :`DamagePreventionChannel` "ECC_PhysicsBody")
          (set `self.blust` true)
          (if (`self.blust`)
            (`self.SetLifeSpan` 3.0)
            (`KismetSystemLibrary.Delay` 3.0)
            (`|SpawnActorFromClass` "BP_Barrel_C" (`KismetMathLibrary.Conv_VectorToTransform` (`self.K2_GetActorLocation`)) "AlwaysSpawn" "OverrideRootScale" null null)))
        (:`then_1`
          (`GameplayStatics.SpawnSoundAtLocation` "/Game/Sounds/Explosion01_Cue.Explosion01_Cue" _returnvalue (struct) 1.0 1.0 0.0 null null))))))

(fn `UserConstructionScript`)