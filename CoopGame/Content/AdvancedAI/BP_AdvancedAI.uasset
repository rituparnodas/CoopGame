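; BP_AdvancedAI is an AI-controlled pawn that can fire and runs the BT_AdvancedAI behavior tree from BeginPlay when it has an AI controller.
; Health changes from HealthComp appear as debug text above the mesh, and Tick calls StopFire every frame while Died is true.
; A disconnected node that sets the player pawn as TargetActor never runs, with a note pointing to AIPerception for that setup.
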(event `self.HealthComp.OnHealthChanged`
  (params (HealthComp :type "SHealthComponent Object Reference") (Health :type "Float (single-precision)") (HealthDelta :type "Float (single-precision)") (DamageType :type "DamageType Object Reference") (InstigatedBy :type "Controller Object Reference") (DamageCauser :type "Actor Object Reference"))
  (`KismetSystemLibrary.DrawDebugString` (+ (`SceneComponent.K2_GetComponentLocation` (`self.Mesh`)) (0.0 0.0 200.0)) (`KismetStringLibrary.Conv_DoubleToString` Health) null (struct :`R` 1.0 :`G` 0.086574 :`A` 1.0) 1.0))

(event `self.ReceiveTick`
  (params (DeltaSeconds :type "Float (single-precision)"))
  (if (`self.bDied`)
    (`self.StopFire`)))

(event `self.ReceiveBeginPlay`
  (bind _returnvalue (`AIBlueprintHelperLibrary.GetAIController` self))
  (`/Engine/EditorBlueprintResources/StandardMacros.IsValid` _returnvalue
    (:`Is Valid`
      (`AIController.RunBehaviorTree` _returnvalue "/Game/AdvancedAI/BT_AdvancedAI.BT_AdvancedAI"))))

(fn `UserConstructionScript`)