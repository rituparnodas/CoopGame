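; Player pawn Blueprint that feeds animation state, manages HUD widgets and switches between first- and third-person cameras.
; On authority or the local client, Tick converts control pitch into a signed, scaled roll rotator and copies jump state; left mouse sets the Fire animation flag.
; Local BeginPlay creates crosshair and health widgets; death removes the health widget, and the GameMode respawn callback creates another.
; Weapon spawning here is unused, having moved to C++.
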(event `self.ReceiveTick`
  (params (DeltaSeconds :type "Float (single-precision)"))
  (bind _pitch (.pitch (`self.GetControlRotation`)))
  ;[0.5124 0 1] Replicating Player Pitch, Jump
  (`|ExecutionSequence`
    (:`then_0`
      (`/Engine/EditorBlueprintResources/ActorMacros.Switch Has Authority`
        (:`Authority`
          (set `self.ControllerPitch` (`KismetMathLibrary.MakeRotator` (/ (`KismetMathLibrary.SelectFloat` (- 360.0 _pitch) (* _pitch -1.0) (> _pitch 180.0)) 3.0)) :!label _label)
          (set `self.SetJump` (`self.bWasJumping`)))))
    (:`then_1`
      (if (`self.IsLocallyControlled`)
        (goto _label)))))

(event `Key|LeftMouseButton`
  (params (Key :type "Key Structure"))
  ;[0 0.405 1] Fire() for Animation
  (:`Pressed`
    (set `self.Fire` true))
  (:`Released`
    (set `self.Fire` false)))

(event `self.HealthComp.OnHealthChanged`
  (params (HealthComp :type "SHealthComponent Object Reference") (Health :type "Float (single-precision)") (HealthDelta :type "Float (single-precision)") (DamageType :type "DamageType Object Reference") (InstigatedBy :type "Controller Object Reference") (DamageCauser :type "Actor Object Reference"))
  (if (<= Health 0.0)
    (`/Engine/EditorBlueprintResources/StandardMacros.IsValid` (stale `self.ReceiveBeginPlay` _returnvalue_2)
      (:`Is Valid`
        (`Widget.RemoveFromParent` (stale `self.ReceiveBeginPlay` _returnvalue_2))))))

(event `self.ReceiveBeginPlay`
  ;[0 1 0] Setup Crosshair And Health Indicator
  (`|ExecutionSequence`
    (:`then_0`
      (bind _asbp_game_mode (cast `/Game/Blueprint/BP_GameMode` (`GameplayStatics.GetGameMode`)))
      (add `SGameMode.OnRespawn` _asbp_game_mode (delegate `OnRespawn_Event_0`)))
    (:`then_1`
      (if (`self.IsLocallyControlled`)
        (`|ExecutionSequence`
          (:`then_0`
            (bind _returnvalue (`|CreateWidget` "/Game/UI/WBP_Crosshair.WBP_Crosshair_C"))
            (`UserWidget.AddToViewport` _returnvalue 0))
          (:`then_1`
            (bind _returnvalue_2 (`|CreateWidget` "/Game/UI/WBP_HealthIndicator.WBP_HealthIndicator_C"))
            (`UserWidget.AddToViewport` _returnvalue_2 0)))))))

(event `OnRespawn_Event_0`
  (bind _returnvalue (`|CreateWidget` "/Game/UI/WBP_HealthIndicator.WBP_HealthIndicator_C"))
  (`UserWidget.AddToViewport` _returnvalue 0))

(event `InputAction|Camera`
  (params (Key :type "Key Structure"))
  ;[0 0.8241 1 1 20] ADS & SwapCamera() V and RMB
  (:`Pressed`
    (`|ExecutionSequence`
      (:`then_0`
        ;[1 1 1] Need RPC For This Later
        (`self.SwapCamera`))
      (:`then_1`
        (`ActorComponent.ToggleActive` (`self.TPPCameraComp`))
        (`ActorComponent.ToggleActive` (`self.FPPCameraComp`))))))

(fn `UserConstructionScript`)