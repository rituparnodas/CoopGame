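; Game mode that spawns AI bots and awards score for kills.
; SpawnNewBot runs an EQS query for a spawn location, draws debug spheres at results and spawns mostly BP_AdvancedAI, occasionally BP_TrackerBot, skipping spawns that would still collide after adjustment.
; An OnActorKilled binding made at BeginPlay adds score to the killer's BP_PlayerState when a non-player pawn dies, then prints the total.
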(event `self.SpawnNewBot`
  ;[1 1 1] Run EQS_Query
  (bind _returnvalue (`EnvQueryManager.RunEQSQuery` "/Game/Blueprint/EQS_FindSpawnLocation.EQS_FindSpawnLocation" self "RandomBest25Pct"))
  (add `EnvQueryInstanceBlueprintWrapper.OnQueryFinishedEvent` _returnvalue (delegate `OnQueryFinishedEvent`)))

(event `OnQueryFinishedEvent`
  (params (QueryInstance :type "EnvQueryInstanceBlueprintWrapper Object Reference") (QueryStatus :type "EEnvQueryStatus Enum" :default "Processing"))
  ;[1 1 1] Run EQS_Query
  (bind _resultlocations (`EnvQueryInstanceBlueprintWrapper.GetQueryResultsAsLocations` QueryInstance))
  (switch `EEnvQueryStatus` QueryStatus
    (:`Success`
      (for _array_element _resultlocations
        (`KismetSystemLibrary.DrawDebugSphere` _array_element 50.0 12 (struct :`R` 1.0 :`G` 0.775803 :`A` 1.0) 2.0 2.0)
        (`|SpawnActorFromClass` (select `bool` (<= (`KismetMathLibrary.RandomFloatInRange` 0.0 100.0) 90.0) :`false` "/Game/Blueprint/BP_TrackerBot.BP_TrackerBot_C" :`true` "/Game/AdvancedAI/BP_AdvancedAI.BP_AdvancedAI_C" :!type "Actor Class Reference") (`KismetMathLibrary.MakeTransform` _array_element) "AdjustIfPossibleButDontSpawnIfColliding" "OverrideRootScale" null null)))))

(event `self.ReceiveBeginPlay`
  ;[1 1 1] Add Score
  (add `self.OnActorKilled` (delegate `OnActorKilledEvent`)))

(event `OnActorKilledEvent` :!signature `self.OnActorKilled`
  (params (VictimActor :type "Actor Object Reference") (KillerActor :type "Actor Object Reference") (KillerController :type "Controller Object Reference"))
  (bind _playerstate (`Pawn.PlayerState` (`Controller.K2_GetPawn` KillerController)))
  ;[1 1 1] Add Score
  (bind _aspawn (cast `Pawn` VictimActor))
  (if (not (`Pawn.IsPlayerControlled` _aspawn))
    (`/Engine/EditorBlueprintResources/StandardMacros.IsValid` KillerController
      (:`Is Valid`
        (`/Engine/EditorBlueprintResources/StandardMacros.IsValid` _playerstate
          (:`Is Valid`
            (bind _asbp_player_state (cast `/Game/Blueprint/BP_PlayerState` _playerstate))
            (`SPlayerState.AddScore` _asbp_player_state 20.0)
            (`KismetSystemLibrary.PrintString` (`KismetStringLibrary.Conv_DoubleToString` (`PlayerState.Score` _asbp_player_state)) true true (struct :`G` 1.0 :`A` 1.0) 5.0)))))))

(fn `UserConstructionScript`)