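; Blueprint for a tracker bot that makes its sound louder the faster it moves.
; Tick maps the bot's velocity magnitude to the volume multiplier of its audio component.
; FindNextPath, a navmesh path query to the player with debug spheres at each point, is unused and marked as moved to C++.
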(event `self.ReceiveBeginPlay`)

(event `FindNextPath`
  ;[0.99 0 0] [Not Using]Moved To C++
  (bind _returnvalue (`NavigationSystemV1.FindPathToActorSynchronously` (`self.K2_GetActorLocation`) (`GameplayStatics.GetPlayerPawn` 0) 50.0 null null))
  (for _array_element (`NavigationPath.PathPoints` _returnvalue)
    (`KismetSystemLibrary.DrawDebugSphere` _array_element 20.0 12 (struct :`G` 0.024614 :`B` 1.0 :`A` 1.0) 2.0 1.0)))

(event `self.ReceiveTick`
  (params (DeltaSeconds :type "Float (single-precision)"))
  (`AudioComponent.SetVolumeMultiplier` (`self.AudioComp`) (`KismetMathLibrary.MapRangeClamped` (`KismetMathLibrary.VSize` (`self.GetVelocity`)) 10.0 1000.0 0.1 5.0)))

(fn `UserConstructionScript`)